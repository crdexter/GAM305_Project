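; Floor actor that takes damage while a BP_BaseEntity stands in its DamageArea, likely a breakable floor.
; Overlap begin and end events toggle a single CauseDamage flag, without counting how many entities are inside.
; While the flag is set, Tick runs through a Delay to apply LevelDamage as radius damage to its own StaticMeshDM at the actor's location roughly every half second.
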(event `self.DamageArea.OnComponentBeginOverlap`
  (params (OverlappedComponent :type "PrimitiveComponent Object Reference") (OtherActor :type "Actor Object Reference") (OtherComp :type "PrimitiveComponent Object Reference") (OtherBodyIndex :type Integer) (bFromSweep :type Boolean) (SweepResult :type "HitResult Structure (by ref)"))
  (cast `/Game/SideScrollerBP/Blueprints/EnemyExperiments/BP_BaseEntity` OtherActor)
  (set `self.CauseDamage?` true))

(event `self.DamageArea.OnComponentEndOverlap`
  (params (OverlappedComponent :type "PrimitiveComponent Object Reference") (OtherActor :type "Actor Object Reference") (OtherComp :type "PrimitiveComponent Object Reference") (OtherBodyIndex :type Integer))
  (cast `/Game/SideScrollerBP/Blueprints/EnemyExperiments/BP_BaseEntity` OtherActor)
  (set `self.CauseDamage?` false))

(event `self.ReceiveTick`
  (params (DeltaSeconds :type "Float (single-precision)"))
  (if (`self.CauseDamage?`)
    (`KismetSystemLibrary.Delay` 0.5)
    (`DestructibleComponent.ApplyRadiusDamage` (`self.StaticMesh_DM`) (`self.LevelDamage`) (`self.K2_GetActorLocation`) 3.0 10.0 false)))

(fn `UserConstructionScript`)