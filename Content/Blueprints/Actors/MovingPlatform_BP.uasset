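; Moving platform actor that slides its static mesh back and forth along a spline after a configurable starting delay.
; The main timeline always starts, using bool flags to pick one of four travel curves and pausing before each run.
; SecondTracks or Last flags additionally start one of two other timelines without those pauses.
; Each timeline maps its curve to spline distance and uses an end flag to alternate play and reverse.
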(event `self.ReceiveBeginPlay`
  ;[1 1 1] Event Start
  (`KismetSystemLibrary.Delay` (`self.StartingDelay`))
  (`self.StartTrack`)
  (if (`self.SecondTracks`)
    (`self.Tracks_2 Start`)
    (elif (`self.Last`)
      (`self.LastTrackStart`))))

(event `StartTrack`
  (bind _returnvalue (`SplineComponent.GetSplineLength` (`self.Spline`)))
  ;[1 1 1] Moving Platforms: simple
  (`KismetSystemLibrary.Delay` 1.0)
  (bind (_direction _travel_a _travel_b _travel_c _travel_d) (`Timeline|TrackMovement` :!label _label)
    (:`Update`
      (if (`self.A_Track`)
        (`SceneComponent.K2_SetWorldLocation` (`self.StaticMesh`) (`SplineComponent.GetLocationAtDistanceAlongSpline` (`self.Spline`) (* _travel_a _returnvalue) "World") false false) ; A
        (elif (`self.B_Track`)
          (`SceneComponent.K2_SetWorldLocation` (`self.StaticMesh`) (`SplineComponent.GetLocationAtDistanceAlongSpline` (`self.Spline`) (* _travel_b _returnvalue) "World") false false) ; B
          (elif (`self.C_Track`)
            (`SceneComponent.K2_SetWorldLocation` (`self.StaticMesh`) (`SplineComponent.GetLocationAtDistanceAlongSpline` (`self.Spline`) (* _travel_c _returnvalue) "World") false false) ; C
            (elif (`self.D_Track`)
              (`SceneComponent.K2_SetWorldLocation` (`self.StaticMesh`) (`SplineComponent.GetLocationAtDistanceAlongSpline` (`self.Spline`) (* _travel_d _returnvalue) "World") false false) ; D
            )))))
    (:`Finished`
      (if (`self.TrackEnd`)
        (set `self.TrackEnd` false)
        (`self.ReverseTrack`)
        (else
          (set `self.TrackEnd` true)
          (`self.StartTrack`))))))

(event `ReverseTrack`
  ;[1 1 1] Moving Platforms: simple
  (`KismetSystemLibrary.Delay` 1.0)
  (goto _label :!via `Reverse`))

(event `Continue`
  ;[1 1 1] Continuous Track
  (bind (_direction _track_ab) (`Timeline|Timeline_0` :!label _label_2)
    (:`Update`
      (`SceneComponent.K2_SetWorldLocation` (`self.StaticMesh`) (`SplineComponent.GetLocationAtDistanceAlongSpline` (`self.Spline`) (* _track_ab (`SplineComponent.GetSplineLength` (`self.Spline`))) "World") false false))
    (:`Finished`
      (if (`self.TrackEnd_2`)
        (set `self.TrackEnd_2` false)
        (`self.Continue`)
        (else
          (set `self.TrackEnd_2` true)
          (`self.Tracks_2 Reverse`))))))

(event `Tracks_2 Start`
  ;[1 1 1] Continuous Track
  (`KismetSystemLibrary.Delay` (`self.StartingDelay`))
  (goto _label_2))

(event `Tracks_2 Reverse`
  ;[1 1 1] Continuous Track
  (goto _label_2 :!via `Reverse`))

(event `LastTrackContinue`
  ;[1 1 1] LastTrack Line
  (bind (_direction _newtrack_0) (`Timeline|LastTrack` :!label _label_3)
    (:`Update`
      (`SceneComponent.K2_SetWorldLocation` (`self.StaticMesh`) (`SplineComponent.GetLocationAtDistanceAlongSpline` (`self.Spline`) (* _newtrack_0 (`SplineComponent.GetSplineLength` (`self.Spline`))) "World") false false))
    (:`Finished`
      (if (`self.LastTrackEnded`)
        (`self.LastTrackReverse`)
        (set `self.LastTrackEnded` false)
        (else
          (`self.LastTrackContinue`)
          (set `self.LastTrackEnded` true))))))

(event `LastTrackStart`
  ;[1 1 1] LastTrack Line
  (goto _label_3))

(event `LastTrackReverse`
  ;[1 1 1] LastTrack Line
  (goto _label_3 :!via `Reverse`))

(fn `UserConstructionScript`)