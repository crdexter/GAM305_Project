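; PlayerProjectile_BP is the player's projectile actor, moved by a ProjectileMovement component.
; FireInDirection sets its velocity from a given direction and the component's initial speed.
; Overlapping a BP_BaseEnemy applies fixed damage, then plays an impact sound and destroys the projectile.
; A blocking hit plays the same sound and destroys it without dealing damage.
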(event `self.Collision.OnComponentHit`
  (params (HitComponent :type "PrimitiveComponent Object Reference") (OtherActor :type "Actor Object Reference") (OtherComp :type "PrimitiveComponent Object Reference") (NormalImpulse :type "Vector Structure") (Hit :type "HitResult Structure (by ref)"))
  (`GameplayStatics.PlaySoundAtLocation` "/Game/Audio/shot_impact_Cue.shot_impact_Cue" (`self.K2_GetActorLocation`) (struct) 1.0 1.0 0.0 null null null)
  (`self.K2_DestroyActor`))

(event `self.Collision.OnComponentBeginOverlap`
  (params (OverlappedComponent :type "PrimitiveComponent Object Reference") (OtherActor :type "Actor Object Reference") (OtherComp :type "PrimitiveComponent Object Reference") (OtherBodyIndex :type Integer) (bFromSweep :type Boolean) (SweepResult :type "HitResult Structure (by ref)"))
  (bind _asbp_base_enemy (cast `/Game/SideScrollerBP/Blueprints/EnemyExperiments/BP_BaseEnemy` OtherActor))
  (`GameplayStatics.ApplyDamage` _asbp_base_enemy 100.0)
  (`GameplayStatics.PlaySoundAtLocation` "/Game/Audio/shot_impact_Cue.shot_impact_Cue" (`self.K2_GetActorLocation`) (struct) 1.0 1.0 0.0 null null null)
  (`self.K2_DestroyActor`))

(fn `FireInDirection`
  (params (`Shoot Direction` :type "Vector Structure (by ref)"))
  (set `MovementComponent.Velocity` (* `Shoot Direction` (`ProjectileMovementComponent.InitialSpeed` (`self.ProjectileMovement`))) (`self.ProjectileMovement`)))

(fn `UserConstructionScript`)