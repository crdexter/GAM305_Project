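; Elevator actor that moves a cylinder platform when the player character enters its trigger box.
; Overlap start waits one second, then plays the Up timeline, which sets the cylinder's relative location from its UpTrack or DownTrack, chosen by the IsUp flag.
; Overlap end waits three seconds, then reverses the same timeline.
; IsUp is only read in these graphs, never changed.
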(event `self.Box.OnComponentBeginOverlap`
  (params (OverlappedComponent :type "PrimitiveComponent Object Reference") (OtherActor :type "Actor Object Reference") (OtherComp :type "PrimitiveComponent Object Reference") (OtherBodyIndex :type Integer) (bFromSweep :type Boolean) (SweepResult :type "HitResult Structure (by ref)"))
  ;[1 1 1] Basic Elevator
  (cast `/Game/SideScrollerBP/Blueprints/EnemyExperiments/BP_PlayerCharacter` OtherActor)
  (`KismetSystemLibrary.Delay` 1.0)
  (bind (_direction _uptrack _downtrack) (`Timeline|Up` :!label _label)
    (:`Update`
      (if (`self.isUp`)
        (`SceneComponent.K2_SetRelativeLocation` (`self.Cylinder`) _downtrack false false) ; Down
        (else
          (`SceneComponent.K2_SetRelativeLocation` (`self.Cylinder`) _uptrack false false) ; Up
        )))))

(event `self.Box.OnComponentEndOverlap`
  (params (OverlappedComponent :type "PrimitiveComponent Object Reference") (OtherActor :type "Actor Object Reference") (OtherComp :type "PrimitiveComponent Object Reference") (OtherBodyIndex :type Integer))
  ;[1 1 1] Basic Elevator
  (cast `/Game/SideScrollerBP/Blueprints/EnemyExperiments/BP_PlayerCharacter` OtherActor)
  (`KismetSystemLibrary.Delay` 3.0)
  (goto _label :!via `Reverse`))

(fn `UserConstructionScript`)